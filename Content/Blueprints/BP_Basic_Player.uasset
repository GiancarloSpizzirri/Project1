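; BP_Basic_Player is a basic player pawn Blueprint that handles movement, jumping and camera look from player input.
; Forward/back and right/left axes feed AddMovementInput along the actor's forward and right vectors, and the Jump action calls Jump on press.
; Look axes drive controller yaw and pitch directly, and the construction script is empty.
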(event Input|ActionEvents|InputActionJump
  (params (Key :type Key%20Structure :default "None"))
  ;[0.3834 0.4114 1] Movement (Jump)
  (:Pressed
    (Character|Jump)))

(event Input|AxisEvents|InputAxisFowards/Backwards
  (params (AxisValue :type Float%20%28single-precision%29))
  ;[0.4826 0.3708 1] Movement (Forward/Back, Right/Left)
  (Pawn|Input|AddMovementInput (Transformation|GetActorForwardVector) AxisValue false))

(event Input|AxisEvents|InputAxisRight/Left
  (params (AxisValue :type Float%20%28single-precision%29))
  ;[0.4826 0.3708 1] Movement (Forward/Back, Right/Left)
  (Pawn|Input|AddMovementInput (Transformation|GetActorRightVector) AxisValue false))

(event Input|AxisEvents|InputAxisLookLeft/Right
  (params (AxisValue :type Float%20%28single-precision%29))
  ;[0.7587 1 0.229] Look (Right/Left, Up/Down)
  (Pawn|Input|AddControllerYawInput AxisValue))

(event Input|AxisEvents|InputAxisLookUp/Down
  (params (AxisValue :type Float%20%28single-precision%29))
  ;[0.7587 1 0.229] Look (Right/Left, Up/Down)
  (Pawn|Input|AddControllerPitchInput AxisValue))

(fn ConstructionScript)